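; SlowTarget is an actor that moves vertically between two positions at timed intervals.
; Tick counts down MoveTimeInterval while idle, then plays the MoveTarget timeline if the actor is exactly at its starting Z, otherwise reverses it.
; The timeline's ZPosition track sets world Z directly rather than as an offset, and its Finished event clears Moving to restart the countdown.
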(event `self.ReceiveBeginPlay`
  (set `self.StartZPosition` (.z (`self.K2_GetActorLocation`)))
  (set `self.TimeSinceLastMove` (`self.MoveTimeInterval`)))

(event `self.ReceiveTick`
  (params (DeltaSeconds :type "Float (single-precision)"))
  (if (not (`self.Moving`))
    (bind _output_get (set `self.TimeSinceLastMove` (- (`self.TimeSinceLastMove`) DeltaSeconds)))
    (if (<= _output_get 0.0)
      (set `self.Moving` true)
      (set `self.TimeSinceLastMove` (`self.MoveTimeInterval`))
      (if (== (.z (`self.K2_GetActorLocation`)) (`self.StartZPosition`))
        (bind (_direction _zposition) (`Timeline|MoveTarget` :!label _label)
          (:`Update`
            (`self.K2_SetActorLocation` (`KismetMathLibrary.MakeVector` (.x (`self.K2_GetActorLocation`)) (.y (`self.K2_GetActorLocation`)) _zposition)))
          (:`Finished`
            (set `self.Moving` false)))
        (else
          (goto _label :!via `Reverse`))))))

(fn `UserConstructionScript`)